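; Interactable tree that drops a leaf or branch pickup-style actor when the Interact event fires.
; A random roll favors BP_leaf over BP_branch at about 65/35, spawning it at a random X/Y offset around the tree at the tree's own height.
; A box trigger shows a widget component while BP_FirstPersonCharacter overlaps it and hides it on exit.
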(event OnComponentBeginOverlap(Box)
  (params (OverlappedComponent :type Primitive%20Component%20Object%20Reference) (OtherActor :type Actor%20Object%20Reference) (OtherComp :type Primitive%20Component%20Object%20Reference) (OtherBodyIndex :type Integer) (bFromSweep :type Boolean) (SweepResult :type Hit%20Result%20Structure%20%28by%20ref%29))
  (Utilities|Casting|CastToBP_FirstPersonCharacter OtherActor)
  (Development|SetHiddeninGame (Variables|Default|GetWidget) false false))

(event OnComponentEndOverlap(Box)
  (params (OverlappedComponent :type Primitive%20Component%20Object%20Reference) (OtherActor :type Actor%20Object%20Reference) (OtherComp :type Primitive%20Component%20Object%20Reference) (OtherBodyIndex :type Integer))
  (Utilities|Casting|CastToBP_FirstPersonCharacter OtherActor)
  (Development|SetHiddeninGame (Variables|Default|GetWidget) true false))

(event EventInteract
  (bind _returnvalue (Transformation|GetActorLocation))
  (bind (_x _y _z) (Math|Vector|BreakVector _returnvalue))
  (bind _returnvalue_2 (+ _x 2.5e+02))
  (bind _returnvalue_3 (- _x 2.5e+02))
  (bind _returnvalue_4 (+ _y 2.5e+02))
  (bind _returnvalue_5 (- _y 2.5e+02))
  (bind _returnvalue_6 (Math|Random|RandomFloatinRange _returnvalue_3 _returnvalue_2))
  (bind _returnvalue_7 (Math|Random|RandomFloatinRange _returnvalue_5 _returnvalue_4))
  (bind _returnvalue_8 (Math|Vector|MakeVector _returnvalue_6 _returnvalue_7 _z))
  (bind _returnvalue_9 (Math|Conversions|ToTransform(Vector) _returnvalue_8))
  (if (>= (Math|Random|RandomFloatinRange 0.0 1e+01) 3.5)
    (Game|SpawnActorfromClass "/Game/Blueprints/BP_leaf.BP_leaf_C" _returnvalue_9 "Undefined" "MultiplyWithRoot" 0 0)
    (else
      (Game|SpawnActorfromClass "/Game/Blueprints/BP_branch.BP_branch_C" _returnvalue_9 "Undefined" "MultiplyWithRoot" 0 0))))

(fn ConstructionScript)